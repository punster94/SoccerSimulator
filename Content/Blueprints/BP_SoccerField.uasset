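; Soccer field actor that runs the match camera, publishes play-area bounds to a material parameter collection and controls global time dilation.
; Each tick the camera eases after the ball, shrinking its offset and blending toward per-goal rotations near either end.
; OnGoal plays a timeline-driven time-dilation effect; debug keys adjust, trigger or toggle dilation.
; Wall-hit events are empty, leaving the ResetBall recentering function unwired.
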(event OnComponentHit(TopWall)
  (params (HitComponent :type Primitive%20Component%20Object%20Reference) (OtherActor :type Actor%20Object%20Reference) (OtherComp :type Primitive%20Component%20Object%20Reference) (NormalImpulse :type Vector) (Hit :type Hit%20Result%20Structure%20%28by%20ref%29)))

(event OnComponentHit(BottomWall)
  (params (HitComponent :type Primitive%20Component%20Object%20Reference) (OtherActor :type Actor%20Object%20Reference) (OtherComp :type Primitive%20Component%20Object%20Reference) (NormalImpulse :type Vector) (Hit :type Hit%20Result%20Structure%20%28by%20ref%29)))

(event OnComponentHit(LeftWall)
  (params (HitComponent :type Primitive%20Component%20Object%20Reference) (OtherActor :type Actor%20Object%20Reference) (OtherComp :type Primitive%20Component%20Object%20Reference) (NormalImpulse :type Vector) (Hit :type Hit%20Result%20Structure%20%28by%20ref%29)))

(event OnComponentHit(RightWall)
  (params (HitComponent :type Primitive%20Component%20Object%20Reference) (OtherActor :type Actor%20Object%20Reference) (OtherComp :type Primitive%20Component%20Object%20Reference) (NormalImpulse :type Vector) (Hit :type Hit%20Result%20Structure%20%28by%20ref%29)))

(event Custom|EmphasizeGoal
  (bind _dialation (Timeline|TimeDialationTimeline PlayFromStart)
    (:Update
      (Utilities|Time|SetGlobalTimeDilation (* (Variables|Default|GetTimeDialationOnPlay) _dialation)))
    (:Finished
      (Utilities|Time|SetGlobalTimeDilation (Variables|Default|GetTimeDialationOnPlay)))))

(event EventBeginPlay
  (bind _returnvalue (Transformation|GetActorLocation))
  (Input|EnableInput (Game|GetPlayerController 0))
  (Utilities|Time|SetGlobalTimeDilation (Variables|Default|GetTimeDialationOnPlay))
  (bind _output_get (Variables|Default|SetCamera (Variables|/Script/Engine.ChildActorComponent|GetChildActor (Variables|Default|GetCameraActor))))
  (Transformation|SetActorLocationAndRotation _output_get (+ (Variables|Default|GetInitialCameraPosition) _returnvalue) (Variables|Default|GetInitialCameraRotation))
  (Game|Player|SetViewTargetwithBlend (Game|GetPlayerController 0) _output_get 0.0 "VTBlend_Linear" 0.0 false)
  (Variables|Default|SetDistanceFromGoal (Math|Float|Absolute(Float) (- (.x (Transformation|GetActorLocation (Variables|/Script/Engine.ChildActorComponent|GetChildActor (Variables|Default|GetBlueGoalComponent)))) (.X (Math|Vector|BreakVector _returnvalue))))))

(event Collision|EventActorBeginOverlap
  (params (OtherActor :type Actor%20Object%20Reference)))

(event EventTick
  (params (DeltaSeconds :type Float%20%28single-precision%29))
  (bind _camera (Variables|Default|GetCamera))
  (bind _playarea (Variables|Default|GetPlayArea))
  (bind _bluegoalcomponent (Variables|Default|GetBlueGoalComponent))
  (bind _distancefromgoaltorotate (Variables|Default|GetDistanceFromGoalToRotate))
  (bind _soccerballcomponent (Variables|Default|GetSoccerBallComponent))
  (bind _childactor (Variables|/Script/Engine.ChildActorComponent|GetChildActor _bluegoalcomponent))
  (bind _childactor_2 (Variables|/Script/Engine.ChildActorComponent|GetChildActor _soccerballcomponent))
  (bind _returnvalue (Transformation|GetActorLocation _childactor))
  (bind _returnvalue_2 (Transformation|GetActorLocation _childactor_2))
  (bind _returnvalue_3 (- _returnvalue_2 _returnvalue))
  (bind _returnvalue_4 (Math|Float|Absolute(Float) (.x _returnvalue_3)))
  (Rendering|Material|SetVectorParameterValue "/Game/Materials/M_ParameterLibrary.M_ParameterLibrary" "PlayAreaLocation" (Math|Conversions|ToLinearColor(Vector) (Transformation|GetWorldLocation _playarea)) :!class /Script/Engine.KismetMaterialLibrary)
  (Rendering|Material|SetVectorParameterValue "/Game/Materials/M_ParameterLibrary.M_ParameterLibrary" "PlayAreaScaledBounds" (Math|Conversions|ToLinearColor(Vector) (Components|Box|GetScaledBoxExtent _playarea)) :!class /Script/Engine.KismetMaterialLibrary)
  (Transformation|SetActorLocation _camera (Math|Vector|Lerp(Vector) (Transformation|GetActorLocation _camera) (+ _returnvalue_2 (* (Variables|Default|GetCameraBallOffset) (- 1.0 (Math|Float|Clamp(Float) (/ (Math|Float|Absolute(Float) (.x (- _returnvalue_2 (Transformation|GetActorLocation)))) (Variables|Default|GetDistanceFromGoal)) 0.0 (Variables|Default|GetMinimumCameraDistanceRatio))))) (Variables|Default|GetCameraBlendAlpha)) false false)
  (if (<= _returnvalue_4 (Variables|Default|GetDistanceFromGoal))
    (Variables|Default|SetTargetCameraRotation (Math|Rotator|Lerp(Rotator) (Variables|Default|GetBlueGoalRotation) (Variables|Default|GetInitialCameraRotation) (Math|Float|Clamp(Float) (/ _returnvalue_4 _distancefromgoaltorotate))))
    (else
      (Variables|Default|SetTargetCameraRotation (Math|Rotator|Lerp(Rotator) (Variables|Default|GetRedGoalRotation) (Variables|Default|GetInitialCameraRotation) (Math|Float|Clamp(Float) (/ (Math|Float|Absolute(Float) (.x (- _returnvalue_2 (Transformation|GetActorLocation (Variables|/Script/Engine.ChildActorComponent|GetChildActor (Variables|Default|GetRedGoalComponent)))))) _distancefromgoaltorotate))))))
  (bind _output_get (Variables|Default|SetCurrentCameraRotation (Math|Rotator|Lerp(Rotator) (Variables|Default|GetCurrentCameraRotation) (Variables|Default|GetTargetCameraRotation) (Variables|Default|GetCameraBlendAlpha))))
  (Transformation|SetActorRotation _camera _output_get))

(event EventOnGoal
  (CallFunction|EmphasizeGoal))

(event Input|KeyboardEvents|Home
  (params (Key :type Key%20Structure :default "AnyKey"))
  (:Pressed
    (bind _output_get (Variables|Default|SetTimeDialationOnPlay (+ (Variables|Default|GetTimeDialationOnPlay) 0.1)))
    (Utilities|Time|SetGlobalTimeDilation _output_get)
    (Development|PrintString (Utilities|String|Append "Time Dialation: " (Utilities|String|ToString(Float) _output_get)) true true "(R=1.000000,G=0.085170,B=0.204911,A=1.000000)")))

(event Input|KeyboardEvents|End
  (params (Key :type Key%20Structure :default "AnyKey"))
  (:Pressed
    (bind _output_get (Variables|Default|SetTimeDialationOnPlay (+ (Variables|Default|GetTimeDialationOnPlay) -0.1)))
    (Utilities|Time|SetGlobalTimeDilation _output_get)
    (Development|PrintString (Utilities|String|Append "Time Dialation: " (Utilities|String|ToString(Float) _output_get)) true true "(R=1.000000,G=0.085170,B=0.204911,A=1.000000)")))

(event Input|KeyboardEvents|SpaceBar
  (params (Key :type Key%20Structure :default "AnyKey"))
  (:Pressed
    (Utilities|FlowControl|FlipFlop
      (:A
        (Variables|Default|SetbPaused true)
        (Utilities|Time|SetGlobalTimeDilation 1.0))
      (:B
        (Variables|Default|SetbPaused false)
        (Utilities|Time|SetGlobalTimeDilation (Variables|Default|GetTimeDialationOnPlay))))))

(event Input|KeyboardEvents|Decimal
  (params (Key :type Key%20Structure :default "AnyKey"))
  (:Pressed
    (CallFunction|EmphasizeGoal)))

(fn ConstructionScript)

(fn ResetBall
  (params (Actor :type Actor%20Object%20Reference) (Normal :type Vector))
  (bind _soccerballcomponent (Variables|Default|GetSoccerBallComponent))
  (bind _childactor (Variables|/Script/Engine.ChildActorComponent|GetChildActor _soccerballcomponent))
  (if (== Actor _childactor)
    (bind _asbp_soccer_ball (Utilities|Casting|CastToBP_SoccerBall _childactor)
      (:then
        (Class|SoccerBall|PlaceatPosition _asbp_soccer_ball (+ (Transformation|GetWorldLocation (Variables|Default|GetField)) "0, 0,200.000000"))
        (return))
      (:CastFailed
        (return)))
    (else
      (return))))