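; Red soccer team actor with four child-actor field players.
; On BeginPlay it enables input and caches the BP_SoccerBall in the level.
; PageUp and PageDown toggle a support-spot display flag.
; Unconnected test chains exercise FieldPlayer steering behaviors (Interpose, Pursue, Arrive, Seek, Separate) on each player, but none of them ever run.
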(event EventBeginPlay
  (Input|EnableInput (Game|GetPlayerController 0))
  (bind _outactors (Actor|GetAllActorsOfClass "/Game/Blueprints/BP_SoccerBall.BP_SoccerBall_C"))
  (Variables|Default|SetSoccerBall (Utilities|Array|Get(acopy) _outactors)))

(event Collision|EventActorBeginOverlap
  (params (OtherActor :type Actor%20Object%20Reference)))

(event EventTick
  (params (DeltaSeconds :type Float%20%28single-precision%29)))

(event Input|KeyboardEvents|4
  (params (Key :type Key%20Structure :default "AnyKey")))

(event Input|KeyboardEvents|PageUp
  (params (Key :type Key%20Structure :default "AnyKey"))
  (:Pressed
    (Variables|Default|SetDisplaySupportSpots true)))

(event Input|KeyboardEvents|PageDown
  (params (Key :type Key%20Structure :default "AnyKey"))
  (:Pressed
    (Variables|Default|SetDisplaySupportSpots false)))

(event Input|KeyboardEvents|Q
  (params (Key :type Key%20Structure :default "AnyKey")))

(event Input|KeyboardEvents|W
  (params (Key :type Key%20Structure :default "AnyKey")))

(event Input|KeyboardEvents|E
  (params (Key :type Key%20Structure :default "AnyKey")))

(event Input|KeyboardEvents|R
  (params (Key :type Key%20Structure :default "AnyKey")))

(event Input|KeyboardEvents|Z
  (params (Key :type Key%20Structure :default "AnyKey")))

(event Input|KeyboardEvents|X
  (params (Key :type Key%20Structure :default "AnyKey")))

(event Input|KeyboardEvents|C
  (params (Key :type Key%20Structure :default "AnyKey")))

(event Input|KeyboardEvents|V
  (params (Key :type Key%20Structure :default "AnyKey")))

(event Input|KeyboardEvents|1
  (params (Key :type Key%20Structure :default "AnyKey")))

(event Input|KeyboardEvents|2
  (params (Key :type Key%20Structure :default "AnyKey")))

(event Input|KeyboardEvents|A
  (params (Key :type Key%20Structure :default "AnyKey")))

(event Input|KeyboardEvents|S
  (params (Key :type Key%20Structure :default "AnyKey")))

(event Input|KeyboardEvents|D
  (params (Key :type Key%20Structure :default "AnyKey")))

(event Input|KeyboardEvents|F
  (params (Key :type Key%20Structure :default "AnyKey")))

(event Input|KeyboardEvents|T
  (params (Key :type Key%20Structure :default "AnyKey")))

(event Input|KeyboardEvents|Y
  (params (Key :type Key%20Structure :default "AnyKey")))

(event Input|KeyboardEvents|U
  (params (Key :type Key%20Structure :default "AnyKey")))

(event Input|KeyboardEvents|I
  (params (Key :type Key%20Structure :default "AnyKey")))

(event Input|KeyboardEvents|3
  (params (Key :type Key%20Structure :default "AnyKey")))

(fn ConstructionScript)