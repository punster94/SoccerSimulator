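; Soccer ball actor that can be pushed around with debug keyboard controls.
; On BeginPlay it enables input from player controller 0.
; Each arrow key calls Kick with a fixed world-axis direction and DebugMovespeed as the force.
; Disconnected SetPhysicsLinearVelocity nodes on BallMesh remain in the graph but never run.
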(event EventBeginPlay
  (Input|EnableInput (Game|GetPlayerController 0)))

(event Collision|EventActorBeginOverlap
  (params (OtherActor :type Actor%20Object%20Reference)))

(event EventTick
  (params (DeltaSeconds :type Float%20%28single-precision%29)))

(event Input|KeyboardEvents|Up
  (params (Key :type Key%20Structure :default "AnyKey"))
  (:Pressed
    (Class|SoccerBall|Kick "0,-1.000000, 0" (Variables|Default|GetDebugMovespeed))))

(event Input|KeyboardEvents|Down
  (params (Key :type Key%20Structure :default "AnyKey"))
  (:Pressed
    (Class|SoccerBall|Kick "0,1.000000, 0" (Variables|Default|GetDebugMovespeed))))

(event Input|KeyboardEvents|Right
  (params (Key :type Key%20Structure :default "AnyKey"))
  (:Pressed
    (Class|SoccerBall|Kick "1.000000, 0, 0" (Variables|Default|GetDebugMovespeed))))

(event Input|KeyboardEvents|Left
  (params (Key :type Key%20Structure :default "AnyKey"))
  (:Pressed
    (Class|SoccerBall|Kick "-1.000000,0.000000, 0" (Variables|Default|GetDebugMovespeed))))

(fn ConstructionScript)